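; An actor with its own health that loses a hit's worth each time the third-person player character overlaps it.
; On BeginPlay it binds an overlap handler, which filters for BP_ThirdPersonCharacter with a cast.
; Each valid overlap subtracts DamagePerHit from CurrentHealth, prints the new value, and destroys the actor once health drops below one.
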(event `self.ReceiveBeginPlay`
  (add `self.ActorDelegate` (delegate `OnBeginOverlap`)))

(event `OnBeginOverlap` :!signature `self.ActorDelegate`
  (params (OverlappedComponent :type "PrimitiveComponent Object Reference") (OtherActor :type "Actor Object Reference") (OtherComp :type "PrimitiveComponent Object Reference") (OtherBodyIndex :type Integer) (bFromSweep :type Boolean) (SweepResult :type "HitResult Structure (by ref)"))
  (cast `/Game/ThirdPerson/Blueprints/BP_ThirdPersonCharacter` OtherActor)
  (bind _output_get (set `self.CurrentHealth` (- (`self.CurrentHealth`) (`self.DamagePerHit`))))
  (`KismetSystemLibrary.PrintString` (`KismetStringLibrary.Conv_IntToString` _output_get))
  (`/Engine/EditorBlueprintResources/StandardMacros.CompareInt` _output_get 1
    (:`<`
      (`self.K2_DestroyActor`))))

(fn `UserConstructionScript`)