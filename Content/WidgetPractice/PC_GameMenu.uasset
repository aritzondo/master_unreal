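; Player controller, judging by its PC_ name, that routes the open-menu input to the player character's UI in a widget practice setup.
; When the Enhanced Input action IA_OpenMenu starts, it gets the UI from the character and calls MenuButtonClicked on it.
; GetPlayer lazily caches the first BP_ThirdPersonCharacter found in the level through GetAllActorsOfClass rather than using the possessed pawn.
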(event `EnhancedInput|/Game/ThirdPerson/Input/Actions/IA_OpenMenu`
  (params (ActionValue :type Boolean) (ElapsedSeconds :type "Float (double-precision)") (TriggeredSeconds :type "Float (double-precision)") (InputAction :type "InputAction Object Reference" :default "/Game/ThirdPerson/Input/Actions/IA_OpenMenu.IA_OpenMenu"))
  (:`Started`
    (`/Game/WidgetPractice/UI/WB_GameUI.MenuButtonClicked` (`/Game/ThirdPerson/Blueprints/BP_ThirdPersonCharacter.GetMyUI` (`self.GetPlayer`)))))

(fn `GetPlayer`
  (returns (Player :type "/Game/ThirdPerson/Blueprints/BP_ThirdPersonCharacter Object Reference"))
  (`/Engine/EditorBlueprintResources/StandardMacros.IsValid` (`self.playerChar`)
    (:`Is Valid`
      _)
    (:`Is Not Valid`
      (bind _outactors (`GameplayStatics.GetAllActorsOfClass` "/Game/ThirdPerson/Blueprints/BP_ThirdPersonCharacter.BP_ThirdPersonCharacter_C"))
      (set `self.playerChar` (`|GetArrayItem` _outactors))))
  (return (`self.playerChar`)))

(fn `UserConstructionScript`)